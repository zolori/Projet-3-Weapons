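; AC_FloatingAnimation is an actor component that makes its owning actor bob up and down while spinning in place.
; On BeginPlay it caches the owner's transform as a baseline.
; Each tick it accumulates time and sets the owner's transform from that baseline, adding a sine-based Z offset scaled by MaxOffsetZ and a continuous yaw from RotationSpeed, leaving other components unchanged.
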(event `self.ReceiveBeginPlay`
  (set `self.initTransform` (`Actor.GetTransform` (`self.GetOwner`))))

(event `self.ReceiveTick`
  (params (DeltaSeconds :type "Float (single-precision)"))
  (bind _inittransform (`self.initTransform`))
  (bind _time (`self.time`))
  (set `self.time` (+ DeltaSeconds _time))
  (`Actor.K2_SetActorTransform` (`self.GetOwner`) (`KismetMathLibrary.MakeTransform` (`KismetMathLibrary.MakeVector` (.x (.location _inittransform)) (.y (.location _inittransform)) (+ (* (`KismetMathLibrary.Sin` _time) (`self.maxOffsetZ`)) (.z (.location _inittransform)))) (`KismetMathLibrary.MakeRotator` (.roll (.rotation _inittransform)) (.pitch (.rotation _inittransform)) (+ (* _time (`self.rotationSpeed`)) (.yaw (.rotation _inittransform)))) (.scale _inittransform)) false false))