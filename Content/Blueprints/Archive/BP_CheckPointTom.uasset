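; BP_CheckPointTom is a checkpoint actor with a box trigger, left with its checkpoint logic unfinished.
; BeginPlay caches BP_GamemodeTom and the player character, then tests CheckpointOrder for zero with nothing following.
; Box overlap prints a debug string and compares the other actor to the player, but takes no further action.
; The calls that report this checkpoint to the game mode through UpdateCheckpoint are disconnected and never run.
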(event `self.ReceiveBeginPlay`
  (bind _asbp_gamemode_tom (cast `/Game/Blueprints/Archive/BP_GamemodeTom` (`GameplayStatics.GetGameMode`)))
  (set `self.Gamemode` _asbp_gamemode_tom)
  (set `self.playerCharacter` (`GameplayStatics.GetPlayerCharacter` 0))
  (if (== (`self.CheckpointOrder`) 0)
    _))

(event `self.Box.OnComponentBeginOverlap`
  (params (OverlappedComponent :type "PrimitiveComponent Object Reference") (OtherActor :type "Actor Object Reference") (OtherComp :type "PrimitiveComponent Object Reference") (OtherBodyIndex :type Integer) (bFromSweep :type Boolean) (SweepResult :type "HitResult Structure (by ref)"))
  (`KismetSystemLibrary.PrintString` "Hello")
  (if (== OtherActor (`self.playerCharacter`))
    _))

(fn `UserConstructionScript`)