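; Electric weapon that locks onto a hostile creature by line trace and charges it with an arc while fire is held.
; Tick builds the charge and shifts the creature's dynamic material BodyColor from yellow to white.
; At maximum charge, it damages the target and hostile creatures in range at one-third damage, while a timeline scales an explosion sphere.
; Charge resets only on a new hit, so this repeats each tick until firing stops.
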(event `self.ReceiveBeginPlay`
  (`parent.ReceiveBeginPlay`)
  (`SceneComponent.SetVisibility` (`self.ElectricArc`) false false)
  (set `self.PlayerCharacter` (`GameplayStatics.GetPlayerPawn` 0))
  (set `self.PlayerController` (`GameplayStatics.GetPlayerController` 0)))

(event `self.ReceiveTick`
  (params (DeltaSeconds :type "Float (single-precision)"))
  (bind _electricityexplosionrange (`self.ElectricityExplosionRange`))
  (bind _targetedcreature (`self.TargetedCreature`))
  (`parent.ReceiveTick` DeltaSeconds)
  (`/Engine/EditorBlueprintResources/StandardMacros.IsValid` (`self.TargetedCreature`)
    (:`Is Valid`
      (if (`SceneComponent.IsVisible` (`self.ElectricArc`))
        (bind _output_get (set `self.ElectricCharge` (+ DeltaSeconds (`self.ElectricCharge`))))
        (`MaterialInstanceDynamic.SetVectorParameterValue` (`self.MaterialCreature`) "BodyColor" (make `LinearColor` 1.0 1.0 (`KismetMathLibrary.Lerp` 0.0 1.0 (/ _output_get (`self.MaxElectricCharge`))) 1.0))
        (if (>= (`self.ElectricCharge`) (`self.MaxElectricCharge`))
          (`/Game/Blueprints/Characters/BP_HostileCreature.UpdateLife` _targetedcreature (`self.Damage`))
          (bind _outactors (`KismetSystemLibrary.SphereOverlapActors` (`self.K2_GetActorLocation` _targetedcreature) _electricityexplosionrange (`|MakeArray` "ObjectTypeQuery3" :!type "EObjectTypeQuery Enum") "/Game/Blueprints/Characters/BP_HostileCreature.BP_HostileCreature_C"))
          (for _array_element _outactors
            (bind _asbp_hostile_creature (cast `/Game/Blueprints/Characters/BP_HostileCreature` _array_element))
            (`/Game/Blueprints/Characters/BP_HostileCreature.UpdateLife` _asbp_hostile_creature (/ (`self.Damage`) 3.0)))
          (bind (_direction _lerp_alpha) (`Timeline|Timeline_0` :!via `PlayFromStart`)
            (:`Update`
              (bind _returnvalue (`KismetMathLibrary.Lerp` 0.0 _electricityexplosionrange _lerp_alpha))
              (`SceneComponent.SetWorldScale3D` (`self.Electric explosion sphere`) (`KismetMathLibrary.MakeVector` _returnvalue _returnvalue _returnvalue)))))))))

(event `self.BeginFiring`
  (bind _returnvalue (`self.K2_GetActorLocation` (`self.PlayerCharacter`)))
  (bind (_outhit _returnvalue_2) (`KismetSystemLibrary.LineTraceSingle` :`Start` _returnvalue :`End` (+ _returnvalue (* (`KismetMathLibrary.GetForwardVector` (`Controller.GetControlRotation` (`self.PlayerController`))) (`self.range`))) :`TraceChannel` "TraceTypeQuery1" :`bTraceComplex` true :`DrawDebugType` "ForDuration"))
  (if _returnvalue_2
    (bind _asbp_hostile_creature (cast `/Game/Blueprints/Characters/BP_HostileCreature` (`.HitActor` (`GameplayStatics.BreakHitResult` _outhit)))
      (:`then`
        (bind _output_get (set `self.TargetedCreature` _asbp_hostile_creature))
        (bind _returnvalue_3 (`PrimitiveComponent.CreateDynamicMaterialInstance` (`Character.Mesh` _output_get) 0 null "None"))
        (set `self.MaterialCreature` _returnvalue_3)
        (set `self.ElectricCharge` 0.0)
        (`SceneComponent.SetVisibility` (`self.ElectricArc`) true false))
      (:`CastFailed`
        (`KismetSystemLibrary.PrintString` "Oups")))
    (else
      (`KismetSystemLibrary.PrintString` "Raté"))))

(event `self.StopFiring`
  (`SceneComponent.SetVisibility` (`self.ElectricArc`) false false))

(fn `UserConstructionScript`
  (`parent.UserConstructionScript`))