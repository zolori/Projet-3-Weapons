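; Game mode Blueprint that manages player lives, checkpoint respawning and game over for a first-person game.
; On BeginPlay it caches the FirstPersonCharacter, and UpdateCheckpoint stores whichever checkpoint it receives, as its validity check changes nothing.
; RespawnPlayer spends a life to teleport the player to that checkpoint and align control rotation, or calls GameOver when none remain.
; The GameOver event resets lives and checkpoint and reopens the Proto level, while Restart calls ResetLevel.
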(event `self.ReceiveBeginPlay`
  (`self.RegisterPlayer`))

(event `GameOver`
  (`KismetSystemLibrary.PrintText` "Game over !")
  (set `self.PlayerLife` 3)
  ;[1 1 1] resetting checkpoint
  (set `self.PlayerCheckpoint` null)
  (`GameplayStatics.OpenLevelBySoftObjectPtr` "/Game/Maps/Proto.Proto"))

(fn `Game Over`)

(fn `RegisterPlayer`
  (bind _asfirst_person_character (cast `/Game/Blueprints/FirstPersonCharacter` (`GameplayStatics.GetPlayerCharacter` 0)))
  (set `self.PlayerCharacter` _asfirst_person_character)
  (return))

(fn `RespawnPlayer`
  (bind _playerlife (`self.PlayerLife`))
  (bind (_returnvalue_location _returnvalue_rotation) (`KismetMathLibrary.BreakTransform` (`self.GetTransform` (`self.PlayerCheckpoint`))))
  (if (> _playerlife 0)
    (`/Engine/EditorBlueprintResources/StandardMacros.DecrementInt` _playerlife
      (:`  `
        (`self.K2_TeleportTo` (`self.PlayerCharacter`) _returnvalue_location _returnvalue_rotation)
        (`Controller.SetControlRotation` (`GameplayStatics.GetPlayerController` 0) _returnvalue_rotation)))
    (else
      (`self.Game Over`)))
  (return))

(fn `Restart`
  (`self.ResetLevel`))

(fn `Update Checkpoint`
  (params (Checkpoint :type "/Game/Blueprints/BP_CheckPoint Object Reference"))
  (`/Engine/EditorBlueprintResources/StandardMacros.IsValid` (`self.PlayerCheckpoint`)
    (:`Is Valid`
      (if true
        (`KismetSystemLibrary.PrintString` "set" :!label _label)
        (set `self.PlayerCheckpoint` Checkpoint)))
    (:`Is Not Valid`
      (goto _label)))
  (return))

(fn `UserConstructionScript`)