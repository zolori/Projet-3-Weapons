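; BP_Grappin is a grappling hook launcher that fires a hook with a visible cable.
; BeginFiring toggles it: it either destroys the live hook and cable, or spawns a BP_Hook at the player pawn, launched by impulse along camera forward.
; A gravity-free cable component is added at runtime and attached to the hook, with its end offset updated on Tick.
; RemoveCable destroys only the cable.
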(event `self.ReceiveTick`
  (params (DeltaSeconds :type "Float (single-precision)"))
  (bind _currcable (`self.CurrCable`))
  (`parent.ReceiveTick` DeltaSeconds)
  (`/Engine/EditorBlueprintResources/StandardMacros.IsValid` _currcable
    (:`Is Valid`
      (`/Engine/EditorBlueprintResources/StandardMacros.IsValid` (`self.CurrHook`)
        (:`Is Valid`
          (set `CableComponent.EndLocation` (- (`SceneComponent.K2_GetComponentLocation` (`Actor.RootComponent` (`self.CurrHook`))) (`SceneComponent.K2_GetComponentLocation` (`Actor.RootComponent` (`GameplayStatics.GetPlayerPawn` 0)))) _currcable))))))

(event `self.BeginFiring`
  (bind _currhook (`self.CurrHook`))
  (`/Engine/EditorBlueprintResources/StandardMacros.IsValid` _currhook
    (:`Is Valid`
      (`self.K2_DestroyActor` _currhook)
      (`ActorComponent.K2_DestroyComponent` (`self.CurrCable`)))
    (:`Is Not Valid`
      (bind _returnvalue (`|SpawnActorFromClass` "/Game/Blueprints/BP_Hook.BP_Hook_C" (`KismetMathLibrary.MakeTransform` (`self.K2_GetActorLocation` (`GameplayStatics.GetPlayerPawn` 0)) (struct) (0.2 0.2 0.2)) "Undefined" "OverrideRootScale" null null))
      (bind _output_get (set `self.CurrHook` _returnvalue))
      (`PrimitiveComponent.AddImpulse` (`/Game/Blueprints/BP_Hook.Sphere` _output_get) (* (`self.GetActorForwardVector` (`GameplayStatics.GetPlayerCameraManager` 0)) 80.0) "None" false)
      (bind _returnvalue_2 (`AddComponent|NODE_AddCableComponent-0`))
      (`PrimitiveComponent.SetEnableGravity` _returnvalue_2 false)
      (bind _output_get_2 (set `self.CurrCable` _returnvalue_2))
      (`CableComponent.SetAttachEndTo` _output_get_2 (`self.CurrHook`) "None" "None"))))

(event `RemoveCable`
  (`ActorComponent.K2_DestroyComponent` (`self.CurrCable`)))

(fn `UserConstructionScript`
  (`parent.UserConstructionScript`))