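; Game mode that tracks the player's last checkpoint and handles respawning the first-person character.
; On BeginPlay it caches the FirstPersonCharacter and seeds LastCheckPoint from the player pawn's location.
; RespawnPlayer moves the character's root to that transform, sets control rotation from a fixed rotator transformed by the checkpoint, and zeroes movement velocity, printing debug strings along the way.
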(event `self.ReceiveBeginPlay`
  (bind _returnvalue (`GameplayStatics.GetActorOfClass` "/Game/FirstPersonBP/Blueprints/FirstPersonCharacter.FirstPersonCharacter_C"))
  (set `self.Player` _returnvalue)
  (set `self.LastCheckPoint` (`KismetMathLibrary.Conv_VectorToTransform` (`self.K2_GetActorLocation` (`GameplayStatics.GetPlayerPawn` 0)))))

(event `RespawnPlayer`
  (bind _player (`self.Player`))
  (bind _lastcheckpoint (`self.LastCheckPoint`))
  (`KismetSystemLibrary.PrintString` "world transform")
  (`SceneComponent.K2_SetWorldTransform` (`Actor.RootComponent` (`self.Player`)) _lastcheckpoint false false)
  (`KismetSystemLibrary.PrintString` "control rotation")
  (`Controller.SetControlRotation` (`Pawn.GetController` _player) (`KismetMathLibrary.TransformRotation` _lastcheckpoint (struct :`Pitch` 90.0 :`Yaw` 90.0 :`Roll` 90.0)))
  (set `MovementComponent.Velocity` (0.0 0.0 0.0) (`Character.CharacterMovement` _player)))

(fn `UserConstructionScript`)