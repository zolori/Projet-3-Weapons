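; BP_PlatformTrigger is a trigger button that makes a linked Platform actor appear and become solid.
; On BeginPlay it hides the activated button component and, if Platform is valid, hides that actor and disables its collision.
; Any overlap with the Box swaps the button to its activated look and restores the platform's visibility and collision, with no logic to revert it.
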(event `self.ReceiveBeginPlay`
  (bind _platform (`self.Platform`))
  (`SceneComponent.SetVisibility` (`self.Pl_button_Activated`) false false)
  (`/Engine/EditorBlueprintResources/StandardMacros.IsValid` _platform
    (:`Is Valid`
      (`self.SetActorEnableCollision` _platform false)
      (`self.SetActorHiddenInGame` _platform true))))

(event `self.Box.OnComponentBeginOverlap`
  (params (OverlappedComponent :type "PrimitiveComponent Object Reference") (OtherActor :type "Actor Object Reference") (OtherComp :type "PrimitiveComponent Object Reference") (OtherBodyIndex :type Integer) (bFromSweep :type Boolean) (SweepResult :type "HitResult Structure (by ref)"))
  (bind _platform (`self.Platform`))
  (`SceneComponent.SetVisibility` (`self.Pl_button_Activated`) true false)
  (`SceneComponent.SetVisibility` (`self.Pl_button_NotActivated`) false false)
  (`/Engine/EditorBlueprintResources/StandardMacros.IsValid` _platform
    (:`Is Valid`
      (`self.SetActorEnableCollision` _platform true)
      (`self.SetActorHiddenInGame` _platform false))))

(fn `UserConstructionScript`)