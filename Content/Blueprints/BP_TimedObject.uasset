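; BP_TimedObject toggles a referenced TimedActor's visibility and collision on a timed cycle after an initial delay.
; Tick waits InitDelay once, then delays by the current Periods entry before calling ShowHide, which flips both states.
; BeginPlay also requests a looping ShowHide timer, with no interval shown.
; NextPeriod increments and wraps PeriodIndex but calls itself unconditionally, and nothing else calls it, so the period index never advances.
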(event `self.ReceiveBeginPlay`
  (`KismetSystemLibrary.K2_SetTimer` null "ShowHide" 0.0 true (`self.InitDelay`)))

(event `self.ReceiveTick`
  (params (DeltaSeconds :type "Float (single-precision)"))
  (if (not (`self.IsInitiated`))
    (`KismetSystemLibrary.Delay` (`self.InitDelay`))
    (set `self.IsInitiated` true))
  (`KismetSystemLibrary.Delay` (`|GetArrayItem` (`self.Periods`) (`self.PeriodIndex`)))
  (`self.ShowHide`))

(fn `NextPeriod`
  (bind _result (`/Engine/EditorBlueprintResources/StandardMacros.IncrementInt` (`self.PeriodIndex`))
    (:`  `
      (if (>= _result (`KismetArrayLibrary.Array_Length` (`self.Periods`)))
        (set `self.PeriodIndex` 0))
      (`self.NextPeriod`)
      (return))))

(fn `ShowHide`
  (bind _timedactor (`self.TimedActor`))
  (`self.SetActorHiddenInGame` _timedactor (not (`Actor.bHidden` _timedactor)))
  (`self.SetActorEnableCollision` _timedactor (not (`self.GetActorEnableCollision` _timedactor)))
  (return))

(fn `UserConstructionScript`)