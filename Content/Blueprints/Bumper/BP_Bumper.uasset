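; BP_Bumper is a firing Blueprint that launches BP_ProjectileBumper toward the point the player's camera is aimed at.
; BeginFiring line traces on Visibility from the player camera along its forward vector up to Range.
; On a hit, it spawns the projectile and passes the hit location as its Direction; a miss spawns nothing.
; A Repulsion spawn at the impact point is left unconnected, and Speed is unused.
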(event `self.BeginFiring`
  (bind _returnvalue (`GameplayStatics.GetPlayerCameraManager` 0))
  (bind _returnvalue_2 (`PlayerCameraManager.GetCameraLocation` _returnvalue))
  (bind (_outhit _returnvalue_3) (`KismetSystemLibrary.LineTraceSingle` _returnvalue_2 (+ _returnvalue_2 (* (`self.GetActorForwardVector` _returnvalue) (`self.range`))) "TraceTypeQuery1"))
  (if _returnvalue_3
    (`|SpawnActorFromClass` "/Game/Blueprints/Bumper/BP_ProjectileBumper.BP_ProjectileBumper_C" (struct) "Undefined" "OverrideRootScale" null (`.Location` (`GameplayStatics.BreakHitResult` _outhit)) null)))

(fn `UserConstructionScript`
  (`parent.UserConstructionScript`))