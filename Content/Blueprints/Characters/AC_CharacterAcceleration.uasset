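; Character component that appears intended as a timed acceleration effect, but currently only sets walk speed and body color.
; BeginPlay creates a dynamic material on the owner's skeletal mesh, sets a base walk speed and loops ChangeSpeed every EffectDuration.
; ChangeSpeed picks the accelerated or default BodyColor from Running, but each branch reassigns the same value, so it never toggles.
; The AccelerationFactor speed calculations are unconnected.
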(event `self.ReceiveBeginPlay`
  (bind _output_get (set `self.Parent` (`self.GetOwner`)))
  (bind _returnvalue (`Actor.GetComponentByClass` _output_get "/Script/Engine.SkeletalMeshComponent"))
  (bind _returnvalue_2 (`PrimitiveComponent.CreateDynamicMaterialInstance` _returnvalue 0 (`PrimitiveComponent.GetMaterial` _returnvalue 0) "None"))
  (set `self.MI_CharacterBody` _returnvalue_2)
  (set `CharacterMovementComponent.MaxWalkSpeed` 300.0 (`Actor.GetComponentByClass` (`self.Parent`) "/Script/Engine.CharacterMovementComponent"))
  (`KismetSystemLibrary.K2_SetTimerDelegate` (delegate `ChangeSpeed`) (`self.EffectDuration`) true))

(event `ChangeSpeed`
  (if (`self.Running`)
    (`MaterialInstanceDynamic.SetVectorParameterValue` (`self.MI_CharacterBody`) "BodyColor" (`self.AccelerationColor`))
    (set `self.Running` true)
    (else
      (`MaterialInstanceDynamic.SetVectorParameterValue` (`self.MI_CharacterBody`) "BodyColor" (`self.DefaultColor`))
      (set `self.Running` false))))