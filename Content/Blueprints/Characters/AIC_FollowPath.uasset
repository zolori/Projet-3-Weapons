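; AI controller that patrols a character along BP_AIPath points and chases the player whenever the player's location projects onto the navmesh.
; BeginPlay fills an Order-indexed array with the path points that lie on navigable space.
; Tick runs the navigation check, switching between running pursuit and walking patrol, with no sight sensing involved.
; NextPoint advances the looping route when an external caller passes the current point's order during patrol.
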(event `self.ReceiveBeginPlay`
  ;[1 1 1] init variable and path
  (set `self.playerCharacter` (`GameplayStatics.GetPlayerCharacter` 0))
  (bind _ascharacter (cast `Character` (`self.K2_GetPawn`)))
  (set `self.controlledCharacter` _ascharacter)
  (bind _outactors (`GameplayStatics.GetAllActorsOfClass` "/Game/Blueprints/Characters/BP_AIPath.BP_AIPath_C"))
  (for _array_element _outactors
    (if (`.ReturnValue` (`NavigationSystemV1.K2_ProjectPointToNavigation` (`self.K2_GetActorLocation` _array_element)))
      (`KismetArrayLibrary.Array_Set` (`self.PathPoints`) (`/Game/Blueprints/Characters/BP_AIPath.order` _array_element) _array_element true))))

(event `self.ReceiveTick`
  (params (DeltaSeconds :type "Float (single-precision)"))
  (bind _playercharacter (`self.playerCharacter`))
  (bind (_projectedlocation _returnvalue) (`NavigationSystemV1.K2_ProjectPointToNavigation` (`self.K2_GetActorLocation` _playercharacter)))
  ;[1 1 1] Patrolling but following player if able to
  (if (`self.IsPatrolling`)
    (if _returnvalue
      (set `CharacterMovementComponent.MaxWalkSpeed` (`self.runningSpeed`) (`Character.CharacterMovement` (`self.controlledCharacter`)))
      (`self.MoveToActor` _playercharacter -1.0 true true true null :!label _label)
      (set `self.IsPatrolling` false))
    (elif _returnvalue
      (goto _label)
      (else
        (`self.Go to Point`)
        (set `self.IsPatrolling` true)))))

(fn `GetPointOrder`
  (returns (PointOrder :type Integer))
  (return (`/Game/Blueprints/Characters/BP_AIPath.order` (`|GetArrayItem` (`self.PathPoints`) (`self.currentPathPoint`)))))

(fn `Go to Point`
  (set `CharacterMovementComponent.MaxWalkSpeed` (`self.walkingSpeed`) (`Character.CharacterMovement` (`self.controlledCharacter`)))
  (`self.MoveToActor` (`|GetArrayItem` (`self.PathPoints`) (`self.currentPathPoint`)) -1.0 true true true null)
  (return))

(fn `Next Point`
  (params (PointCaller :type Integer))
  (if (and (== PointCaller (`self.GetPointOrder`)) (`self.IsPatrolling`))
    (bind _result (`/Engine/EditorBlueprintResources/StandardMacros.IncrementInt` (`self.currentPathPoint`))
      (:`  `
        (if (> _result (`KismetArrayLibrary.Array_LastIndex` (`self.PathPoints`)))
          (set `self.currentPathPoint` 0))
        (`self.Go to Point`)
        (return)))))

(fn `UserConstructionScript`)