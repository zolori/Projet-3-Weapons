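; BP_HostileCreature is an enemy character with a life value that leaves a key behind when it dies.
; UpdateLife adds a signed delta to Life and calls Die once it reaches zero or below.
; Die detaches the controller, waits a few seconds, destroys the actor, then spawns BP_Key lowered by a multiple of BaseEyeHeight.
; BeginPlay caches the player's FirstPersonCharacter, which this file does not otherwise use.
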(event `self.ReceiveBeginPlay`
  (bind _asfirst_person_character (cast `/Game/Blueprints/FirstPersonCharacter` (`GameplayStatics.GetPlayerCharacter` 0)))
  (set `self.CharacterPlayer` _asfirst_person_character))

(event `Die`
  (`self.DetachFromControllerPendingDestroy`)
  (`KismetSystemLibrary.Delay` 5.0)
  (`self.K2_DestroyActor`)
  (`|SpawnActorFromClass` "/Game/Blueprints/Part_1/BP_Key.BP_Key_C" (`KismetMathLibrary.Conv_VectorToTransform` (- (`self.K2_GetActorLocation`) (`KismetMathLibrary.MakeVector` 0.0 0.0 (* 5 (`self.BaseEyeHeight`))))) "Undefined" "OverrideRootScale" null null))

(fn `UpdateLife`
  (params (DeltaLife :type "Float (double-precision)"))
  (bind _output_get (set `self.Life` (+ DeltaLife (`self.Life`))))
  (if (<= _output_get 0.0)
    (`self.Die`))
  (return))

(fn `UserConstructionScript`)