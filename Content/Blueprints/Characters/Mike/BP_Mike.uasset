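; BP_Mike is a character Blueprint that tracks its own health and whether the player is nearby.
; BeginPlay sets Life and MaxLife, and Tick flags IsDead once Life reaches zero or below.
; Tick also compares its distance to player pawn 0 against a fixed radius to set IsNearPlayer, with a trailing Delay that drives nothing.
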(event `self.ReceiveBeginPlay`
  (`parent.ReceiveBeginPlay`)
  (bind _output_get (set `self.Life` 100.0))
  (set `self.MaxLife` _output_get))

(event `self.ReceiveTick`
  (params (DeltaSeconds :type "Float (single-precision)"))
  (`|ExecutionSequence`
    (:`then_0`
      (if (<= (`self.Life`) 0.0)
        (set `self.isDead` true)))
    (:`then_1`
      (if (< 550.0 (`KismetMathLibrary.Vector_Distance` (`self.K2_GetActorLocation` (`GameplayStatics.GetPlayerPawn` 0)) (`self.K2_GetActorLocation`)))
        (set `self.isNearPlayer` false)
        (else
          (set `self.isNearPlayer` true)
          (`KismetSystemLibrary.Delay` 0.5))))))

(fn `UserConstructionScript`)