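; Cactus enemy NPC that shoots spikes at the player's first-person character while it is in range.
; The AttackRange overlap sets or clears the target and the attack flag on the cactus Animation Blueprint.
; A one-second Delay on Tick throttles firing, spawning a Spike, pushing it toward the target by impulse and rotating it to face them.
; Death sets the animation's dead flag, which stops firing, calls the parent logic and plays a sound.
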(event `self.Die`
  (set `/Game/Blueprints/Characters/Cactus/ABP_Cactus.isDead` true (`self.BP_Anim`))
  (`parent.Die`)
  (`GameplayStatics.PlaySound2D` "/Game/ThirdParty/Sounds/Unity_Western_Template/SFX_CactusDeath03.SFX_CactusDeath03" 1.0 1.0 0.0 null null))

(event `self.ReceiveBeginPlay`
  (`parent.ReceiveBeginPlay`)
  (bind _asabp_cactus (cast `/Game/Blueprints/Characters/Cactus/ABP_Cactus` (`SkeletalMeshComponent.GetAnimInstance` (`self.Mesh`))))
  (set `self.BP_Anim` _asabp_cactus))

(event `self.AttackRange.OnComponentBeginOverlap`
  (params (OverlappedComponent :type "PrimitiveComponent Object Reference") (OtherActor :type "Actor Object Reference") (OtherComp :type "PrimitiveComponent Object Reference") (OtherBodyIndex :type Integer) (bFromSweep :type Boolean) (SweepResult :type "HitResult Structure (by ref)"))
  (bind _asfirst_person_character (cast `/Game/Blueprints/Characters/FirstPersonCharacter` OtherActor))
  (set `self.Cible` _asfirst_person_character)
  (set `/Game/Blueprints/Characters/Cactus/ABP_Cactus.isAttacking` true (`self.BP_Anim`)))

(event `self.AttackRange.OnComponentEndOverlap`
  (params (OverlappedComponent :type "PrimitiveComponent Object Reference") (OtherActor :type "Actor Object Reference") (OtherComp :type "PrimitiveComponent Object Reference") (OtherBodyIndex :type Integer))
  (bind _asfirst_person_character (cast `/Game/Blueprints/Characters/FirstPersonCharacter` OtherActor))
  (if (== (`self.Cible`) _asfirst_person_character)
    (set `self.Cible` null)
    (set `/Game/Blueprints/Characters/Cactus/ABP_Cactus.isAttacking` false (`self.BP_Anim`))))

(event `self.ReceiveTick`
  (params (DeltaSeconds :type "Float (single-precision)"))
  (`KismetSystemLibrary.Delay` 1.0)
  (if (not (`/Game/Blueprints/Characters/Cactus/ABP_Cactus.isDead` (`self.BP_Anim`)))
    (`/Engine/EditorBlueprintResources/StandardMacros.IsValid` (`self.Cible`)
      (:`Is Valid`
        (bind _returnvalue (`|SpawnActorFromClass` "/Game/Blueprints/Characters/Cactus/Spike.Spike_C" (`self.GetTransform`) "AlwaysSpawn" "OverrideRootScale" null null))
        (bind _sphere (`/Game/Blueprints/Characters/Cactus/Spike.Sphere` _returnvalue))
        (`PrimitiveComponent.AddImpulse` _sphere (* (`KismetMathLibrary.Normal` (- (`self.K2_GetActorLocation` (`self.Cible`)) (`self.K2_GetActorLocation`))) 7.0) "None" false)
        (`SceneComponent.K2_SetWorldRotation` _sphere (`KismetMathLibrary.FindLookAtRotation` (`self.K2_GetActorLocation`) (`SceneComponent.K2_GetComponentLocation` (`Actor.RootComponent` (`self.Cible`)))) false false)))))

(fn `UserConstructionScript`)