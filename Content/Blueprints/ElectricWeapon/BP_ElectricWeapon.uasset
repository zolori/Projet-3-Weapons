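; Beam weapon that electrifies hostile creatures until they set off an area explosion.
; While firing, a camera line trace steers the laser and picks the target, whose charge builds each tick while other creatures' charges decay.
; Per-creature maps track charge and Niagara particles, whose spawn count scales with charge.
; At max charge, the explosion damages the target, deals reduced damage and partial charge to nearby creatures, and expands a timeline-scaled sphere.
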(event `self.ReceiveBeginPlay`
  ;[1 1 1] initiatialization of variables and components
  (`parent.ReceiveBeginPlay`)
  (`SceneComponent.SetVisibility` (`self.P_Laser_04`) false false)
  (bind _output_get (set `self.PlayerCharacter` (`GameplayStatics.GetPlayerPawn` 0)))
  (set `self.PlayerCamera` (`self.GetComponentByClass` _output_get "/Script/Engine.CameraComponent"))
  (`SceneComponent.K2_DetachFromComponent` (`self.Electric explosion sphere`) "KeepWorld" "KeepWorld" "KeepWorld" false))

(event `self.ReceiveTick`
  (params (DeltaSeconds :type "Float (single-precision)"))
  (bind _p_laser_04 (`self.P_Laser_04`))
  (bind _playercamera (`self.PlayerCamera`))
  (bind _targetedcreature (`self.TargetedCreature`))
  (bind _electrifiedcreatureselectriccharge (`self.ElectrifiedCreaturesElectricCharge`))
  (bind _returnvalue (`SceneComponent.K2_GetComponentLocation` _playercamera))
  ;[1 1 1] updates electric charges of  previous trageted  creature  and their visual effect
  (bind _keys (`BlueprintMapLibrary.Map_Keys` (`self.ElectrifiedCreaturesElectricCharge`)))
  (for _array_element _keys
    (if (== _targetedcreature _array_element)
      (bind _hasmaxedoutelectriccharge (`self.Update Electric Charge` _targetedcreature DeltaSeconds))
      (if _hasmaxedoutelectriccharge
        (`self.ElectricExplosion`))
      (else
        (`self.Update Electric Charge` _array_element (- 0.0 DeltaSeconds)))))
  ;[1 1 1] updating current target
  (`/Engine/EditorBlueprintResources/StandardMacros.Gate` true :!label _label
    (:`Exit`
      (bind (_outhit _returnvalue_2) (`KismetSystemLibrary.LineTraceSingle` _returnvalue (+ _returnvalue (* (`SceneComponent.GetForwardVector` _playercamera) (`self.range`))) "TraceTypeQuery1" true))
      (if _returnvalue_2
        (bind (_bblockinghit _binitialoverlap _time _distance _location _impactpoint _normal _impactnormal _physmat _hitactor _hitcomponent _hitbonename _hititem _elementindex _faceindex _tracestart _traceend) (`GameplayStatics.BreakHitResult` _outhit))
        (`NiagaraComponent.SetVariableVec3` _p_laser_04 "End" _location)
        (if (not (== (`self.TargetedCreature`) _hitactor))
          (bind _asbp_hostile_creature (cast `/Game/Blueprints/Characters/BP_HostileCreature` _hitactor))
          (bind _output_get (set `self.TargetedCreature` _asbp_hostile_creature))
          (if (not (`BlueprintMapLibrary.Map_Contains` _electrifiedcreatureselectriccharge _output_get))
            (`BlueprintMapLibrary.Map_Add` _electrifiedcreatureselectriccharge _output_get)
            (`self.ActivateElectricParticles` _output_get)))
        (else
          (`NiagaraComponent.SetVariableVec3` _p_laser_04 "End" _traceend))))))

(event `self.BeginFiring`
  (`SceneComponent.SetVisibility` (`self.P_Laser_04`) true false)
  (goto _label :!via `Open`))

(event `self.StopFiring`
  (set `self.TargetedCreature` null)
  (`SceneComponent.SetVisibility` (`self.P_Laser_04`) false false)
  (goto _label :!via `Close`))

(event `ElectricExplosion`
  (bind _targetedcreature (`self.TargetedCreature`))
  (bind _electricityexplosionrange (`self.ElectricityExplosionRange`))
  (bind _damage (`self.Damage`))
  (bind _electric_explosion_sphere (`self.Electric explosion sphere`))
  (bind _returnvalue (`self.K2_GetActorLocation` _targetedcreature))
  ;[1 1 1] Getting all enemies in the explosion zone
  (bind _outactors (`KismetSystemLibrary.SphereOverlapActors` _returnvalue _electricityexplosionrange (`|MakeArray` "ObjectTypeQuery3" :!type "EObjectTypeQuery Enum")))
  (for _array_element _outactors
    (if (== _targetedcreature _array_element)
      ;[1 1 1] Target damage
      (`SceneComponent.K2_SetWorldLocation` (`self.Electric explosion sphere`) _returnvalue false false)
      (`/Game/Blueprints/Characters/BP_HostileCreature.UpdateLife` _targetedcreature _damage)
      (if (`self.IsActorBeingDestroyed` _targetedcreature)
        (`BlueprintMapLibrary.Map_Remove` (`self.ElectrifiedCreaturesElectricCharge`) _targetedcreature)
        (`BlueprintMapLibrary.Map_Remove` (`self.ElectrifiedCreatureParticles`) _targetedcreature))
      (else
        ;[1 1 1] Zone damage + partially electrify enemy nearby
        (bind _asbp_hostile_creature (cast `/Game/Blueprints/Characters/BP_HostileCreature` _array_element))
        (`/Game/Blueprints/Characters/BP_HostileCreature.UpdateLife` _asbp_hostile_creature (/ _damage 3.0))
        (`BlueprintMapLibrary.Map_Add` (`self.ElectrifiedCreaturesElectricCharge`) _asbp_hostile_creature (/ (`self.MaxElectricCharge`) 1.5))
        (`self.ActivateElectricParticles` _asbp_hostile_creature))))
  ;[1 1 1] Visual effect of the electric explosion
  (set `self.TargetedCreature` null)
  (`SceneComponent.SetVisibility` _electric_explosion_sphere true false)
  (bind (_direction _lerp_alpha) (`Timeline|Timeline_0` :!via `PlayFromStart`)
    (:`Update`
      (bind _returnvalue_2 (`KismetMathLibrary.Lerp` 0.0 (/ _electricityexplosionrange 100.0) _lerp_alpha))
      (`SceneComponent.SetWorldScale3D` _electric_explosion_sphere (`KismetMathLibrary.MakeVector` _returnvalue_2 _returnvalue_2 _returnvalue_2)))
    (:`Finished`
      (`SceneComponent.SetVisibility` _electric_explosion_sphere false false))))

(fn `ActivateElectricParticles`
  (params (Creature :type "/Game/Blueprints/Characters/BP_HostileCreature Object Reference"))
  (bind _electrifiedcreatureparticles (`self.ElectrifiedCreatureParticles`))
  (bind (_value _returnvalue) (`BlueprintMapLibrary.Map_Find` _electrifiedcreatureparticles Creature))
  (if _returnvalue
    (`ActorComponent.Activate` _value true)
    (else
      (bind _returnvalue_2 (`AddComponent|NODE_AddNiagaraComponent-3` :`self` Creature))
      (`BlueprintMapLibrary.Map_Add` _electrifiedcreatureparticles Creature _returnvalue_2)))
  (return))

(fn `GetElectricParticleCount`
  (params (ElectricCharge :type "Float (double-precision)"))
  (returns (ParticleCount :type Integer))
  (return (`KismetMathLibrary.FTrunc` (`KismetMathLibrary.Lerp` 1.0 10.0 (/ ElectricCharge (`self.MaxElectricCharge`))))))

(fn `Update Electric Charge`
  (params (Creature :type "/Game/Blueprints/Characters/BP_HostileCreature Object Reference") (DeltaCharge :type "Float (double-precision)"))
  (returns (HasMaxedOutElectricCharge :type Boolean))
  (bind _electrifiedcreatureselectriccharge (`self.ElectrifiedCreaturesElectricCharge`))
  (bind _value (`BlueprintMapLibrary.Map_Find` (`self.ElectrifiedCreatureParticles`) Creature))
  (bind _returnvalue (+ (`BlueprintMapLibrary.Map_Find` _electrifiedcreatureselectriccharge Creature) DeltaCharge))
  (`BlueprintMapLibrary.Map_Add` _electrifiedcreatureselectriccharge Creature _returnvalue)
  (`self.UpdateElectricFeedBack` Creature)
  (if (> _returnvalue 0.0)
    (if (> _returnvalue (`self.MaxElectricCharge`))
      (`BlueprintMapLibrary.Map_Add` _electrifiedcreatureselectriccharge Creature)
      (return true)
      (else
        _))
    (else
      (`BlueprintMapLibrary.Map_Remove` _electrifiedcreatureselectriccharge Creature)
      (`/Engine/EditorBlueprintResources/StandardMacros.IsValid` _value
        (:`Is Valid`
          (`ActorComponent.Deactivate` _value))
        (:`Is Not Valid`
          _))))
  (return false))

(fn `UpdateElectricFeedBack`
  (params (Creature :type "/Game/Blueprints/Characters/BP_HostileCreature Object Reference"))
  (bind _value (`BlueprintMapLibrary.Map_Find` (`self.ElectrifiedCreatureParticles`) Creature))
  (bind _particlecount (`self.GetElectricParticleCount` (`BlueprintMapLibrary.Map_Find` (`self.ElectrifiedCreaturesElectricCharge`) Creature)))
  (`/Engine/EditorBlueprintResources/StandardMacros.IsValid` _value
    (:`Is Valid`
      (`NiagaraComponent.SetVariableInt` _value "Minimum_Spawn Count" _particlecount)
      (`NiagaraComponent.SetVariableInt` _value "Maximum_Spawn Count" (+ _particlecount 1)))
    (:`Is Not Valid`
      _))
  (return))

(fn `UserConstructionScript`
  (`parent.UserConstructionScript`))