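; NPC Blueprint for a cactus enemy that shoots spikes at the first-person player while they are within its attack range.
; AttackRange overlaps set or clear the target and toggle the attacking flag on the cactus Animation Blueprint.
; A Delay on Tick throttles firing to about once per second.
; Each shot spawns a Spike, pushes it toward the target with an impulse, and rotates both mesh and spike to face it.
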(event `self.ReceiveBeginPlay`
  (bind _asabp_cactus (cast `/Game/Blueprints/Characters/Cactus/ABP_Cactus` (`SkeletalMeshComponent.GetAnimInstance` (`self.Mesh`))))
  (set `self.BP_Anim` _asabp_cactus))

(event `self.AttackRange.OnComponentBeginOverlap`
  (params (OverlappedComponent :type "PrimitiveComponent Object Reference") (OtherActor :type "Actor Object Reference") (OtherComp :type "PrimitiveComponent Object Reference") (OtherBodyIndex :type Integer) (bFromSweep :type Boolean) (SweepResult :type "HitResult Structure (by ref)"))
  (bind _asfirst_person_character (cast `/Game/Blueprints/FirstPersonCharacter` OtherActor))
  (set `self.Cible` _asfirst_person_character)
  (set `/Game/Blueprints/Characters/Cactus/ABP_Cactus.isAttacking` true (`self.BP_Anim`)))

(event `self.AttackRange.OnComponentEndOverlap`
  (params (OverlappedComponent :type "PrimitiveComponent Object Reference") (OtherActor :type "Actor Object Reference") (OtherComp :type "PrimitiveComponent Object Reference") (OtherBodyIndex :type Integer))
  (bind _asfirst_person_character (cast `/Game/Blueprints/FirstPersonCharacter` OtherActor))
  (if (== (`self.Cible`) _asfirst_person_character)
    (set `self.Cible` null)
    (set `/Game/Blueprints/Characters/Cactus/ABP_Cactus.isAttacking` false (`self.BP_Anim`))))

(event `self.ReceiveTick`
  (params (DeltaSeconds :type "Float (single-precision)"))
  (`KismetSystemLibrary.Delay` 1.0)
  (`/Engine/EditorBlueprintResources/StandardMacros.IsValid` (`self.Cible`)
    (:`Is Valid`
      (bind _returnvalue (`|SpawnActorFromClass` "/Game/Blueprints/Spike.Spike_C" (`self.GetTransform`) "Undefined" "OverrideRootScale" null null))
      (bind _sphere (`/Game/Blueprints/Spike.Sphere` _returnvalue))
      (`PrimitiveComponent.AddImpulse` _sphere (* (`KismetMathLibrary.Normal` (- (`SceneComponent.K2_GetComponentLocation` (`Actor.RootComponent` (`self.Cible`))) (`SceneComponent.K2_GetComponentLocation` (`self.Mesh`)))) 5.0) "None" false)
      (`SceneComponent.K2_SetWorldRotation` (`self.Mesh`) (`KismetMathLibrary.FindLookAtRotation` (`SceneComponent.K2_GetComponentLocation` _sphere) (`SceneComponent.K2_GetComponentLocation` (`Actor.RootComponent` (`self.Cible`)))) false false)
      (`SceneComponent.K2_SetWorldRotation` _sphere (`KismetMathLibrary.FindLookAtRotation` (`SceneComponent.K2_GetComponentLocation` _sphere) (`SceneComponent.K2_GetComponentLocation` (`Actor.RootComponent` (`self.Cible`)))) false false))))

(fn `UserConstructionScript`)