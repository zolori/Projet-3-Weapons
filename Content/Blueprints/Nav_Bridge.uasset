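; Nav link bridge that launches NPCs across to the link's destination when they reach its smart link.
; On SmartLinkReached, it casts the agent to NPC and calls LaunchCharacter, overriding both horizontal and vertical velocity.
; Horizontal velocity equals the raw offset to the destination, implying a one-second ballistic arc.
; A math expression derives vertical velocity from height difference and half of Gravity, plus a small fixed boost.
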(event EventBeginPlay)

(event Collision|EventActorBeginOverlap
  (params (OtherActor :type Actor%20Object%20Reference)))

(event EventTick
  (params (DeltaSeconds :type Float%20%28single-precision%29)))

(event EventSmartLinkReached
  (params (Agent :type Actor%20Object%20Reference) (Destination :type Vector%20%28by%20ref%29 :default "0, 0, 0"))
  (bind (_x _y _z) (Math|Vector|BreakVector Destination))
  (bind _asnpc (Utilities|Casting|CastToNPC Agent))
  (Character|LaunchCharacter _asnpc (Math|Vector|MakeVector (- _x (.X (Math|Vector|BreakVector (Transformation|GetWorldLocation (Variables|/Script/Engine.Actor|GetRootComponent _asnpc))))) (- _y (.Y (Math|Vector|BreakVector (Transformation|GetWorldLocation (Variables|/Script/Engine.Actor|GetRootComponent _asnpc))))) (+ (|(DestZ-(StartZ-(0.500000*Gravity))) _z (.Z (Math|Vector|BreakVector (Transformation|GetWorldLocation (Variables|/Script/Engine.Actor|GetRootComponent _asnpc)))) (Variables|Default|GetGravity)) 5e+01)) true true))

(fn ConstructionScript)