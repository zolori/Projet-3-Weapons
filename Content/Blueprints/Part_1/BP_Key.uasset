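; BP_Key is a key pickup that the player collects by walking into it.
; On overlap with player pawn 0, it casts to FirstPersonCharacter and sets that character's HaveKey flag.
; It then destroys itself, plays the key sound at its location and spawns the P_Healcharacter particle effect slightly below that point.
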(event `self.ReceiveActorBeginOverlap`
  (params (OtherActor :type "Actor Object Reference"))
  (bind _returnvalue (`GameplayStatics.GetPlayerPawn` 0))
  (bind _returnvalue_2 (`self.K2_GetActorLocation`))
  (if (== OtherActor _returnvalue)
    (bind _asfirst_person_character (cast `/Game/Blueprints/Characters/FirstPersonCharacter` _returnvalue))
    (set `/Game/Blueprints/Characters/FirstPersonCharacter.HaveKey` true _asfirst_person_character)
    (`self.K2_DestroyActor`)
    (`GameplayStatics.PlaySoundAtLocation` "/Game/ThirdParty/Sounds/HourOfCode/SFX_key.SFX_key" _returnvalue_2 (struct) 1.0 1.0 0.0 null null null)
    (`NiagaraFunctionLibrary.SpawnSystemAtLocation` "/Game/ThirdParty/Stylized_VFX_StPack/Particles/P_Healcharacter.P_Healcharacter" (- _returnvalue_2 (`KismetMathLibrary.MakeVector` 0.0 0.0 100.0)))))

(fn `UserConstructionScript`)