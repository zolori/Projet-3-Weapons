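; Grenade launcher weapon Blueprint, still a rough stub that launches no projectile.
; BeginFiring prints a debug label and runs a debug-drawn visibility line trace from the player camera along its forward vector, out to Range.
; On a hit it adds a zero impulse to SkeletalMesh rather than to the hit object, so firing has no physical effect yet.
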(event `self.BeginFiring`
  (bind _returnvalue (`GameplayStatics.GetPlayerCameraManager` 0))
  (bind _returnvalue_2 (`PlayerCameraManager.GetCameraLocation` _returnvalue))
  (`KismetSystemLibrary.PrintString` "grenade" true true (struct :`R` 0.521652 :`G` 1.0 :`B` 0.083097 :`A` 1.0))
  (bind (_outhit _returnvalue_3) (`KismetSystemLibrary.LineTraceSingle` :`Start` _returnvalue_2 :`End` (+ _returnvalue_2 (* (`self.GetActorForwardVector` _returnvalue) (`self.range`))) :`TraceChannel` "TraceTypeQuery1" :`DrawDebugType` "ForDuration" :`TraceColor` (struct :`R` 1.0) :`TraceHitColor` (struct :`R` 0.94275 :`G` 1.0) :`DrawTime` 1.0))
  (if _returnvalue_3
    (`PrimitiveComponent.AddImpulse` (`self.SkeletalMesh`) (0.0 0.0 0.0) "None" false)))

(fn `UserConstructionScript`
  (`parent.UserConstructionScript`))