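; BP_Bumper is a weapon Blueprint that fires BP_ProjectileBumper projectiles.
; BeginFiring spawns a scaled-down projectile at its Sphere component, oriented by the first player's camera rotation rather than the weapon's own.
; A Waiting flag and a short Delay form a cooldown that ignores further fire calls until it expires.
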(event `self.BeginFiring`
  (if (not (== (`self.waiting`) true))
    (`|SpawnActorFromClass` "/Game/Blueprints/Weapons/Bumper/BP_ProjectileBumper.BP_ProjectileBumper_C" (`KismetMathLibrary.MakeTransform` (`SceneComponent.K2_GetComponentLocation` (`self.Sphere`)) (`SceneComponent.K2_GetComponentRotation` (`PlayerCameraManager.TransformComponent` (`GameplayStatics.GetPlayerCameraManager` 0))) (0.1 0.1 0.1)) "Undefined" "OverrideRootScale" null null)
    (set `self.waiting` true)
    (`KismetSystemLibrary.Delay` 1.0)
    (set `self.waiting` false)))

(fn `UserConstructionScript`
  (`parent.UserConstructionScript`))