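; Grappling hook weapon that launches BP_Hook projectiles along the camera view and links them with cable components.
; Primary fire shoots a hook cabled to the weapon, or removes the active hook and cable if one exists.
; Alternate fire shoots a second hook cabled to the first, turns off player attraction on both and releases the pair.
; Tick updates the cable end while it simulates physics, and reset clears the active hook and cable.
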(event `self.ReceiveTick`
  (params (DeltaSeconds :type "Float (single-precision)"))
  (bind _currcable (`self.CurrCable`))
  (`parent.ReceiveTick` DeltaSeconds)
  (`/Engine/EditorBlueprintResources/StandardMacros.IsValid` _currcable
    (:`Is Valid`
      (`/Engine/EditorBlueprintResources/StandardMacros.IsValid` (`self.CurrHook`)
        (:`Is Valid`
          (if (`SceneComponent.IsSimulatingPhysics` _currcable "None")
            (set `CableComponent.EndLocation` (- (`SceneComponent.K2_GetComponentLocation` (`Actor.RootComponent` (`self.CurrHook`))) (`SceneComponent.K2_GetComponentLocation` (`Actor.RootComponent` (`GameplayStatics.GetPlayerPawn` 0)))) _currcable)))))))

(event `AlternateFire`
  (`self.Bottom Shoot`))

(event `self.BeginFiring`
  (bind _currhook (`self.CurrHook`))
  (`/Engine/EditorBlueprintResources/StandardMacros.IsValid` _currhook
    (:`Is Valid`
      (`self.K2_DestroyActor` _currhook)
      (`ActorComponent.K2_DestroyComponent` (`self.CurrCable`)))
    (:`Is Not Valid`
      (`self.headShoot`))))

(event `RemoveCable`
  (`ActorComponent.K2_DestroyComponent` (`self.CurrCable`)))

(event `self.ResetWeapon`
  (bind _currcable (`self.CurrCable`))
  (bind _currhook (`self.CurrHook`))
  (`/Engine/EditorBlueprintResources/StandardMacros.IsValid` _currhook
    (:`Is Valid`
      (`self.K2_DestroyActor` _currhook)
      (`/Engine/EditorBlueprintResources/StandardMacros.IsValid` _currcable
        (:`Is Valid`
          (`ActorComponent.K2_DestroyComponent` _currcable))))))

(fn `Bottom Shoot`
  (bind _returnvalue (`GameplayStatics.GetPlayerCameraManager` 0))
  (bind _returnvalue_2 (`self.GetActorForwardVector` _returnvalue))
  (`/Engine/EditorBlueprintResources/StandardMacros.IsValid` (`self.CurrHook`)
    (:`Is Valid`
      (`ActorComponent.K2_DestroyComponent` (`self.CurrCable`))
      (set `/Game/Blueprints/Weapons/grappin/BP_Hook.AttractPlayer` false (`self.CurrHook`))
      (bind _returnvalue_3 (`|SpawnActorFromClass` "/Game/Blueprints/Weapons/grappin/BP_Hook.BP_Hook_C" (`KismetMathLibrary.MakeTransform` (`self.K2_GetActorLocation`) (`PlayerCameraManager.GetCameraRotation` _returnvalue) (0.3 0.3 0.3)) "Undefined" "OverrideRootScale" null null))
      (set `/Game/Blueprints/Weapons/grappin/BP_Hook.OtherEnd` (`self.CurrHook`) _returnvalue_3)
      (set `/Game/Blueprints/Weapons/grappin/BP_Hook.AttractPlayer` false _returnvalue_3)
      (`PrimitiveComponent.AddImpulse` (`/Game/Blueprints/Weapons/grappin/BP_Hook.Sphere` _returnvalue_3) (* _returnvalue_2 80.0) "None" false)
      (`KismetSystemLibrary.PrintString` (`KismetStringLibrary.Conv_VectorToString` _returnvalue_2))
      (bind _returnvalue_4 (`AddComponent|NODE_AddCableComponent-5` :`self` _returnvalue_3))
      (`PrimitiveComponent.SetCollisionEnabled` _returnvalue_4 "NoCollision")
      (`PrimitiveComponent.SetEnableGravity` _returnvalue_4 false)
      (bind _output_get (set `self.CurrCable` _returnvalue_4))
      (`CableComponent.SetAttachEndTo` _output_get (`self.CurrHook`) "None" "None")
      (set `self.CurrHook` null))))

(fn `headShoot`
  (bind _returnvalue (`GameplayStatics.GetPlayerCameraManager` 0))
  (bind _returnvalue_2 (`|SpawnActorFromClass` "/Game/Blueprints/Weapons/grappin/BP_Hook.BP_Hook_C" (`KismetMathLibrary.MakeTransform` (`self.K2_GetActorLocation`) (`PlayerCameraManager.GetCameraRotation` _returnvalue) (0.3 0.3 0.3)) "Undefined" "OverrideRootScale" null null))
  (bind _output_get (set `self.CurrHook` _returnvalue_2))
  (`PrimitiveComponent.AddImpulse` (`/Game/Blueprints/Weapons/grappin/BP_Hook.Sphere` _output_get) (* (`self.GetActorForwardVector` _returnvalue) 80.0) "None" false)
  (bind _returnvalue_3 (`AddComponent|NODE_AddCableComponent-2`))
  (`PrimitiveComponent.SetEnableGravity` _returnvalue_3 false)
  (bind _output_get_2 (set `self.CurrCable` _returnvalue_3))
  (`CableComponent.SetAttachEndTo` _output_get_2 (`self.CurrHook`) "None" "None"))

(fn `UserConstructionScript`
  (`parent.UserConstructionScript`))