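; BP_Hook is the grappling hook projectile of the BP_Grappin weapon, able to pull the player toward where it sticks.
; Its physics sphere stops simulating when it hits anything but a FirstPersonCharacter.
; Tick removes the cable and destroys the hook if it flies beyond maximum range, or, once anchored with AttractPlayer set, applies distance-scaled force to the player's CharacterMovement.
; Destroying the hook also destroys its OtherEnd actor.
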(event `self.ReceiveDestroyed`
  (bind _otherend (`self.OtherEnd`))
  (`/Engine/EditorBlueprintResources/StandardMacros.IsValid` _otherend
    (:`Is Valid`
      (`self.K2_DestroyActor` _otherend))))

(event `self.ReceiveBeginPlay`
  (bind _asfirst_person_character (cast `/Game/Blueprints/Characters/FirstPersonCharacter` (`GameplayStatics.GetPlayerPawn` 0)))
  (set `self.PC` _asfirst_person_character))

(event `self.ReceiveHit`
  (params (MyComp :type "PrimitiveComponent Object Reference") (Other :type "Actor Object Reference") (OtherComp :type "PrimitiveComponent Object Reference") (bSelfMoved :type Boolean) (HitLocation :type "Vector Structure") (HitNormal :type "Vector Structure") (NormalImpulse :type "Vector Structure") (Hit :type "HitResult Structure (by ref)"))
  (bind _returnvalue (`GameplayStatics.GetPlayerPawn` 0))
  (cast `/Game/Blueprints/Characters/FirstPersonCharacter` Other
    (:`CastFailed`
      (`PrimitiveComponent.SetSimulatePhysics` (`self.Sphere`) false)
      (bind _asfirst_person_character (cast `/Game/Blueprints/Characters/FirstPersonCharacter` _returnvalue))
      (set `self.PC` _asfirst_person_character)
      (set `self.PCCharMove` (`self.GetComponentByClass` _returnvalue "/Script/Engine.CharacterMovementComponent")))))

(event `self.ReceiveTick`
  (params (DeltaSeconds :type "Float (single-precision)"))
  (bind _sphere (`self.Sphere`))
  (bind _pccharmove (`self.PCCharMove`))
  (if (`SceneComponent.IsSimulatingPhysics` _sphere "None")
    (`/Engine/EditorBlueprintResources/StandardMacros.CompareFloat` (`KismetMathLibrary.Vector_Distance` (`SceneComponent.K2_GetComponentLocation` (`Actor.RootComponent` (`GameplayStatics.GetPlayerPawn` 0))) (`SceneComponent.K2_GetComponentLocation` _sphere)) (`self.DistToPlayerMax`)
      (:`>`
        (bind _baseweapon (`/Game/Blueprints/Characters/FirstPersonCharacter.GetCurrentWeapon` (`self.PC`)))
        (bind _asbp_grappin (cast `/Game/Blueprints/Weapons/grappin/BP_Grappin` _baseweapon))
        (`/Game/Blueprints/Weapons/grappin/BP_Grappin.RemoveCable` _asbp_grappin)
        (`self.K2_DestroyActor`)))
    (elif (`self.AttractPlayer`)
      (`/Engine/EditorBlueprintResources/StandardMacros.IsValid` _pccharmove
        (:`Is Valid`
          (`CharacterMovementComponent.AddForce` _pccharmove (* (- (`SceneComponent.K2_GetComponentLocation` _sphere) (`SceneComponent.K2_GetComponentLocation` (`Actor.RootComponent` (`self.PC`)))) 300.0)))))))

(fn `UserConstructionScript`)